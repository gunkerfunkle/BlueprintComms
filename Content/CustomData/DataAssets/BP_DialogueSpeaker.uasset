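; BP_DialogueSpeaker is a trigger that plays dialogue from a DialogueData asset as on-screen debug text.
; When the player character overlaps its Box, a valid DialogueData starts a latent Delay loop that advances CurrentIndex every two seconds and prints that line.
; The index increments before each print and is never reset here, and the inclusive bounds check lets it reach one past the last line.
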(event `self.Box.OnComponentBeginOverlap`
  (params (OverlappedComponent :type "PrimitiveComponent Object Reference") (OtherActor :type "Actor Object Reference") (OtherComp :type "PrimitiveComponent Object Reference") (OtherBodyIndex :type Integer) (bFromSweep :type Boolean) (SweepResult :type "HitResult Structure (by ref)"))
  (if (== OtherActor (`GameplayStatics.GetPlayerCharacter` 0))
    (`/Engine/EditorBlueprintResources/StandardMacros.IsValid` (`self.DialogueData`)
      (:`Is Valid`
        (`KismetSystemLibrary.Delay` 2.0 :!label _label)
        (`/Engine/EditorBlueprintResources/StandardMacros.IncrementInt` (`self.CurrentIndex`)
          (:`  `
            (if (<= (`self.CurrentIndex`) (`KismetArrayLibrary.Array_Length` (`/Game/CustomData/DataAssets/PDA_DialogueSequence.Lines` (`self.DialogueData`))))
              (`KismetSystemLibrary.PrintString` (`KismetTextLibrary.Conv_TextToString` (`|GetArrayItem` (`/Game/CustomData/DataAssets/PDA_DialogueSequence.Lines` (`self.DialogueData`)) (`self.CurrentIndex`))))
              (goto _label))))))))

(fn `UserConstructionScript`)