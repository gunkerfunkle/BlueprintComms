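; BP_DialogueMaster is a data-driven NPC actor that shows a dialogue widget while the player stands near it.
; On BeginPlay it creates WBP_Dialogue, and SetupDialogue uses the NPCToShow enum as the DT_DialogueDataExample row name to fill mesh, name, dialogue text and interact sound.
; The Box adds the widget when the player character enters and removes it on any end overlap.
; The interact sound is stored but never played here.
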(event `self.ReceiveBeginPlay`
  (bind _returnvalue (`|CreateWidget` "/Game/CustomData/UserInterface/WBP_Dialogue.WBP_Dialogue_C"))
  (set `self.DialogueUI` _returnvalue)
  (`self.SetupDialogue`))

(event `self.Box.OnComponentBeginOverlap`
  (params (OverlappedComponent :type "PrimitiveComponent Object Reference") (OtherActor :type "Actor Object Reference") (OtherComp :type "PrimitiveComponent Object Reference") (OtherBodyIndex :type Integer) (bFromSweep :type Boolean) (SweepResult :type "HitResult Structure (by ref)"))
  (if (== OtherActor (`GameplayStatics.GetPlayerCharacter` 0))
    (`UserWidget.AddToViewport` (`self.DialogueUI`) 0)))

(event `self.Box.OnComponentEndOverlap`
  (params (OverlappedComponent :type "PrimitiveComponent Object Reference") (OtherActor :type "Actor Object Reference") (OtherComp :type "PrimitiveComponent Object Reference") (OtherBodyIndex :type Integer))
  (`Widget.RemoveFromParent` (`self.DialogueUI`)))

(fn `SetupDialogue`
  (bind _dialogueui (`self.DialogueUI`))
  (bind _returnvalue (`|GetDataTableRow` "/Game/CustomData/DataTables/DT_DialogueDataExample.DT_DialogueDataExample" (`KismetStringLibrary.Conv_StringToName` (`|GetEnumeratorNameAsString` (`self.NPCToShow`))))
    (:`then`
      (bind (_dialogue _interactsound _npcvisual _npcname) (break `/Game/CustomData/Structs/S_DataExample` _returnvalue))
      (`StaticMeshComponent.SetStaticMesh` (`self.NPCVisible`) _npcvisual)
      (set `self.Interact Sound` _interactsound)
      (`TextBlock.SetText` (`/Game/CustomData/UserInterface/WBP_Dialogue.DialogueText` _dialogueui) (`KismetTextLibrary.Conv_StringToText` _dialogue))
      (`TextBlock.SetText` (`/Game/CustomData/UserInterface/WBP_Dialogue.NPCName` _dialogueui) (`KismetTextLibrary.Conv_StringToText` _npcname)))))

(fn `UserConstructionScript`)