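; Demo sphere actor that shows runtime material changes through dynamic material instances.
; The construction script creates an instance of M_Solid on MatSphere and randomizes its base color, metallic and emissive values.
; The Interactwith event rerolls only the base color.
; An unconnected dissolve chain would swap in M_Dissolve, play a timeline and destroy the actor, but it never runs.
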(event `/Game/Blueprints/Materials/Interface/BPI_Interact.InteractWith`
  ; Random Mats on trace
  (`MaterialInstanceDynamic.SetVectorParameterValue` (`self.DynamicMaterial`) "Base Color" (make `LinearColor` (`KismetMathLibrary.RandomFloatInRange` 0.0 1.0) (`KismetMathLibrary.RandomFloatInRange` 0.0 1.0) (`KismetMathLibrary.RandomFloatInRange` 0.0 1.0) (`KismetMathLibrary.RandomFloatInRange` 0.8 1.0))))

(fn `UserConstructionScript`
  ; Setting a random material. Could replace with random mats out of your list of array mats
  (bind _returnvalue (`PrimitiveComponent.CreateDynamicMaterialInstance` (`self.MatSphere`) 0 "/Game/Blueprints/Materials/M_Solid.M_Solid" "None"))
  (bind _output_get (set `self.DynamicMaterial` _returnvalue))
  (`MaterialInstanceDynamic.SetVectorParameterValue` _output_get "Base Color" (make `LinearColor` (`KismetMathLibrary.RandomFloatInRange` 0.0 1.0) (`KismetMathLibrary.RandomFloatInRange` 0.0 1.0) (`KismetMathLibrary.RandomFloatInRange` 0.0 1.0) (`KismetMathLibrary.RandomFloatInRange` 0.8 1.0)))
  (`MaterialInstanceDynamic.SetScalarParameterValue` _output_get "Metallic" (`KismetMathLibrary.RandomFloatInRange` 0.0 1.0))
  (`MaterialInstanceDynamic.SetScalarParameterValue` _output_get "Emissive" (`KismetMathLibrary.RandomFloatInRange` 0.0 0.3)))