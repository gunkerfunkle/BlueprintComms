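; A changeable tile strip that flags each tile when something hits it.
; On BeginPlay it lays out a row of scaled-up plane instances on one InstancedStaticMesh, stepping along negative world X from BaseLocation.
; A component hit uses the hit item index to set that instance's custom data to 1, allowing per-tile changes without separate actors.
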(event `self.ReceiveBeginPlay`
  (bind (_returnvalue_location _returnvalue_rotation _returnvalue_scale) (`KismetMathLibrary.BreakTransform` (`self.GetTransform`)))
  (`StaticMeshComponent.SetStaticMesh` (`self.InstancedStaticMesh`) "/Engine/BasicShapes/Plane.Plane")
  (for _ (range 11)
    (bind _output_get (set `self.BaseLocation` (+ (`self.BaseLocation`) (-500.0 0.0 0.0))))
    (`InstancedStaticMeshComponent.AddInstance` (`self.InstancedStaticMesh`) (`KismetMathLibrary.MakeTransform` _output_get _returnvalue_rotation (* _returnvalue_scale 5.0)) true)))

(event `self.InstancedStaticMesh.OnComponentHit`
  (params (HitComponent :type "PrimitiveComponent Object Reference") (OtherActor :type "Actor Object Reference") (OtherComp :type "PrimitiveComponent Object Reference") (NormalImpulse :type "Vector Structure") (Hit :type "HitResult Structure (by ref)"))
  (`InstancedStaticMeshComponent.SetCustomDataValue` (`self.InstancedStaticMesh`) (`.HitItem` (`GameplayStatics.BreakHitResult` Hit)) 0 1.0 false))

(fn `UserConstructionScript`)