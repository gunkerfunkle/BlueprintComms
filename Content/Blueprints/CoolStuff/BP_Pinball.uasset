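; BP_Pinball is a player-controlled physics ball that rolls by camera-relative torque from the movement axis inputs.
; Hitting a BP_ChangableTile calls its colour change, and other hits print a debug string.
; ResetPinball zeroes velocity and teleports the ball to the active checkpoint cached from GI_PersistantData, but the fall-height check that calls it is disconnected.
; SpawnRockets is unfinished, only drawing debug line traces around an arrow.
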(event `InputAxis|Move Forward / Backward`
  (params (AxisValue :type "Float (single-precision)"))
  (`PrimitiveComponent.AddTorqueInRadians` (`self.BallMesh`) (* (* AxisValue 5000000.0) (`SceneComponent.GetRightVector` (`self.Camera`))) "None" false))

(event `InputAxis|Move Right / Left`
  (params (AxisValue :type "Float (single-precision)"))
  (bind _result (`/Engine/EditorBlueprintResources/StandardMacros.NegateFloat` (* AxisValue 5000000.0))
    (:`  `
      (`PrimitiveComponent.AddTorqueInRadians` (`self.BallMesh`) (* (`SceneComponent.GetForwardVector` (`self.Camera`)) _result) "None" false))))

(event `self.ReceiveBeginPlay`
  (bind _asgi_persistant_data (cast `/Game/CustomData/GameInstances/GI_PersistantData` (`GameplayStatics.GetGameInstance`)))
  (set `self.As GI Persistant Data` _asgi_persistant_data))

(event `self.ReceiveHit`
  (params (MyComp :type "PrimitiveComponent Object Reference") (Other :type "Actor Object Reference") (OtherComp :type "PrimitiveComponent Object Reference") (bSelfMoved :type Boolean) (HitLocation :type "Vector Structure") (HitNormal :type "Vector Structure") (NormalImpulse :type "Vector Structure") (Hit :type "HitResult Structure (by ref)"))
  (bind _asbp_changable_tile (cast `/Game/Blueprints/Materials/BP_ChangableTile` Other)
    (:`then`
      (`/Game/Blueprints/Materials/BP_ChangableTile.ChangeColour` _asbp_changable_tile 0))
    (:`CastFailed`
      (`KismetSystemLibrary.PrintString` "NotIt"))))

(event `self.ReceiveTick`
  (params (DeltaSeconds :type "Float (single-precision)")))

(fn `ResetPinball`
  (`PrimitiveComponent.SetAllPhysicsLinearVelocity` (`self.BallMesh`) (0.0 0.0 0.0) false)
  (`SceneComponent.K2_SetWorldLocation` (`self.BallMesh`) (`/Game/CustomData/GameInstances/GI_PersistantData.Active Checkpoint` (`self.As GI Persistant Data`)) false true))

(fn `SpawnRockets`
  (bind _returnvalue (`self.K2_GetActorLocation`))
  (bind _arrow (`self.Arrow`))
  (bind _returnvalue_2 (`SceneComponent.GetForwardVector` _arrow))
  (bind _returnvalue_3 (`SceneComponent.GetRightVector` _arrow))
  (bind _returnvalue_4 (`SceneComponent.K2_GetComponentLocation` (`self.Arrow`)))
  (bind _output_get (set `self.RocketLocations` (`|MakeArray` (+ _returnvalue_3 _returnvalue_4) (- _returnvalue_3 _returnvalue_4) (+ _returnvalue_2 _returnvalue_4) (- _returnvalue_2 _returnvalue_4))))
  (for _array_element _output_get
    (`KismetSystemLibrary.LineTraceSingle` :`Start` _returnvalue :`End` (* (+ _returnvalue _array_element) 50) :`TraceChannel` "TraceTypeQuery1" :`DrawDebugType` "Persistent")))

(fn `UserConstructionScript`)