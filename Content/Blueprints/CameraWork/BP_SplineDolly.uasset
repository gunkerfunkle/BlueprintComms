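; BP_SplineDolly is a trigger-driven camera dolly that moves a cine camera along a spline while aiming it at a target actor.
; Any overlap with its box blends player 0's view to the dolly and plays a timeline.
; The timeline track, scaled by spline length, sets the camera's position along the path, and a look-at rotation keeps it facing the target each update.
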(event `StartDolly`
  (bind _spline (`self.Spline`))
  (bind _cinecamera (`self.CineCamera`))
  (`PlayerController.SetViewTargetWithBlend` (`GameplayStatics.GetPlayerController` 0) self 1.5 "VTBlend_Linear" 0.0 false)
  (bind (_direction _dollytrack) (`Timeline|DollyTimeline`)
    (:`Update`
      (`SceneComponent.K2_SetWorldLocation` (`self.CineCamera`) (`SplineComponent.GetLocationAtDistanceAlongSpline` _spline (* _dollytrack (`SplineComponent.GetSplineLength` _spline)) "World") false false)
      (`SceneComponent.K2_SetWorldRotation` _cinecamera (`KismetMathLibrary.FindLookAtRotation` (`SceneComponent.K2_GetComponentLocation` _cinecamera) (`self.K2_GetActorLocation` (`self.TargetActor`))) false false))))

(event `self.Box.OnComponentBeginOverlap`
  (params (OverlappedComponent :type "PrimitiveComponent Object Reference") (OtherActor :type "Actor Object Reference") (OtherComp :type "PrimitiveComponent Object Reference") (OtherBodyIndex :type Integer) (bFromSweep :type Boolean) (SweepResult :type "HitResult Structure (by ref)"))
  (`self.StartDolly`))

(fn `UserConstructionScript`)