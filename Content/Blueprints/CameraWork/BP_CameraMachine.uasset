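; BP_CameraMachine is a world actor that temporarily switches the player's view to a level camera when its collision zone is overlapped.
; Any overlap blends to a random BP_Camera among the first three found, waits briefly, then blends back to the player character.
; On BeginPlay, the HeadBob timeline raises the actor from its start position; a reverse event exists but is not called here.
; SetupData is an empty stub.
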(event `self.ReceiveBeginPlay`
  (set `self.StartPosition` (`self.K2_GetActorLocation`))
  (`self.HeadBobUp`)
  (`self.SetupData`))

(event `HeadBobUp`
  (bind (_startposition_x _startposition_y _startposition_z) (`KismetMathLibrary.BreakVector` (`self.StartPosition`)))
  (bind (_direction _headbobtrack) (`Timeline|HeadBob` :!label _label)
    (:`Update`
      (`self.K2_SetActorLocation` (`KismetMathLibrary.MakeVector` _startposition_x _startposition_y (`KismetMathLibrary.Lerp` _startposition_z (+ _startposition_z 50.0) _headbobtrack))))))

(event `HeadBobDown`
  (goto _label :!via `Reverse`))

(event `self.CollisionZone.OnComponentBeginOverlap`
  (params (OverlappedComponent :type "PrimitiveComponent Object Reference") (OtherActor :type "Actor Object Reference") (OtherComp :type "PrimitiveComponent Object Reference") (OtherBodyIndex :type Integer) (bFromSweep :type Boolean) (SweepResult :type "HitResult Structure (by ref)"))
  (bind _outactors (`GameplayStatics.GetAllActorsOfClass` "/Game/Blueprints/CameraWork/BP_Camera.BP_Camera_C"))
  (bind _output_get (set `self.ParentCamera` _outactors))
  (`PlayerController.SetViewTargetWithBlend` (`GameplayStatics.GetPlayerController` 0) (`|GetArrayItem` _output_get (`KismetMathLibrary.RandomIntegerInRange` 0 2)) 1.5 "VTBlend_Linear" 0.0 false)
  (`KismetSystemLibrary.Delay` 3.0)
  (`PlayerController.SetViewTargetWithBlend` (`GameplayStatics.GetPlayerController` 0) (`GameplayStatics.GetPlayerCharacter` 0) 1.5 "VTBlend_Linear" 0.0 false))

(fn `SetupData`)

(fn `UserConstructionScript`)