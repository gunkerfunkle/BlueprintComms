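; BP_CubeToyText is an overlap-triggered text display that reacts to actors implementing the BPI_CubeToy interface.
; When an actor enters OverlappedArea, it stores the actor, checks for the interface, and either sends CubeToyFunctionMessage and shows CorrectText or shows FailText.
; The construction script sets the TextRender to OGText as the initial message, and no end-overlap handler restores it.
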(event `self.OverlappedArea.OnComponentBeginOverlap`
  (params (OverlappedComponent :type "PrimitiveComponent Object Reference") (OtherActor :type "Actor Object Reference") (OtherComp :type "PrimitiveComponent Object Reference") (OtherBodyIndex :type Integer) (bFromSweep :type Boolean) (SweepResult :type "HitResult Structure (by ref)"))
  (set `self.OverlappedActor` OtherActor)
  (if (`KismetSystemLibrary.DoesImplementInterface` (`self.OverlappedActor`) "/Game/BlueprintInterfaces/BPI_CubeToy.BPI_CubeToy_C")
    (message `/Game/BlueprintInterfaces/BPI_CubeToy.CubeToyFunction` (`self.OverlappedActor`))
    (`TextRenderComponent.K2_SetText` (`self.TextRender`) (`self.CorrectText`))
    (else
      (`TextRenderComponent.K2_SetText` (`self.TextRender`) (`self.FailText`)))))

(fn `UserConstructionScript`
  (`TextRenderComponent.K2_SetText` (`self.TextRender`) (`self.OGText`)))