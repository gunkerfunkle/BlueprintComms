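; BP_PaperToyText is a Blueprint communication example: a text display that reports whether an overlapping actor is the correct object.
; The construction script sets the original text.
; When something enters OverlapArea, it stores that actor and checks it for BPI_PaperToy.
; Implementers receive PaperToyFunctionMessage and the text switches to the correct message, while any other actor shows the fail text.
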(event `self.OverlapArea.OnComponentBeginOverlap`
  (params (OverlappedComponent :type "PrimitiveComponent Object Reference") (OtherActor :type "Actor Object Reference") (OtherComp :type "PrimitiveComponent Object Reference") (OtherBodyIndex :type Integer) (bFromSweep :type Boolean) (SweepResult :type "HitResult Structure (by ref)"))
  ;[1 1 1] Checks what is overlapping the actor we made in this blueprint. If anything, it stores the actor into 'overlapped actor' variable
  (set `self.OverlappedActor` OtherActor)
  (if (`KismetSystemLibrary.DoesImplementInterface` (`self.OverlappedActor`) "/Game/BlueprintInterfaces/BPI_PaperToy.BPI_PaperToy_C")
    ;[1 1 1] If that actor has the interface implemented, fire of the blueprint interface function and connect the target (remember we saved whatever overlapped into the target variable.
    (message `/Game/BlueprintInterfaces/BPI_PaperToy.PaperToyFunction` (`self.OverlappedActor`))
    ;[1 1 1] Set text of this actor to display the correct text
    (`TextRenderComponent.K2_SetText` (`self.TextToDisplay`) (`self.CorrectText`))
    (else
      ;[1 1 1] If it doesn't implement the interface, AKA isn't the correct object. Let the player know.
      (`TextRenderComponent.K2_SetText` (`self.TextToDisplay`) (`self.FailText`)))))

(fn `UserConstructionScript`
  (`TextRenderComponent.K2_SetText` (`self.TextToDisplay`) (`self.OGText`)))